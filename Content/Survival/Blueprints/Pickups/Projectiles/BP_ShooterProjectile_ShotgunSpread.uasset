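; Shotgun spread projectile Blueprint that handles what happens to the projectile after a hit.
; On a Static-mobility component it snaps to the impact point facing into the surface, plays a Wiggle timeline that rolls the mesh, then briefly stays stuck.
; It then drops as a zero-velocity physics object that ignores pawns, and is destroyed after a delay.
; Stationary, movable or invalid hits skip straight to that drop.
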(event `self.BP_OnProjectileHit`
  (params (Hit :type "HitResult Structure (by ref)"))
  (bind (_bblockinghit _binitialoverlap _time _distance _location _impactpoint _normal _impactnormal _physmat _hitactor _hitcomponent) (`GameplayStatics.BreakHitResult` Hit))
  (bind _mesh (`self.Mesh`))
  (`/Engine/EditorBlueprintResources/StandardMacros.IsValid` _hitcomponent
    (:`Is Valid`
      (switch `EComponentMobility` (`SceneComponent.Mobility` _hitcomponent)
        (:`Static`
          (`self.K2_SetActorLocationAndRotation` _location (`KismetMathLibrary.MakeRotFromX` (* _normal -1.0)))
          (bind (_direction _rotation) (`Timeline|Wiggle`)
            (:`Update`
              (`SceneComponent.K2_AddRelativeRotation` (`self.Mesh`) (`KismetMathLibrary.MakeRotator` _rotation) false false))
            (:`Finished`
              (`KismetSystemLibrary.Delay` 3.0)
              (`PrimitiveComponent.SetCollisionProfileName` _mesh "PhysicsActor" true :!label _label)
              (`PrimitiveComponent.SetCollisionResponseToChannel` _mesh "ECC_Pawn" "ECR_Ignore")
              (`PrimitiveComponent.SetSimulatePhysics` _mesh true)
              (`PrimitiveComponent.SetPhysicsLinearVelocity` _mesh (0.0 0.0 0.0) false "None")
              (`KismetSystemLibrary.Delay` 5.0)
              (`self.K2_DestroyActor`))))
        (:`Stationary`
          (goto _label))
        (:`Movable`
          (goto _label))))
    (:`Is Not Valid`
      (goto _label))))

(fn `UserConstructionScript`)